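; BP_DockTrigger is a docking zone that shows the win screen when the player's boat stays docked in it.
; On box overlap, it checks that the BP_BoatChar is under a speed limit and its mesh yaw is within a narrow world-space range, then starts a timer and spawns win particles.
; Timer expiry shows UMG_WinScreen through BP_GameHUD, while leaving the box cancels the timer and destroys the particles.
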(event OnComponentBeginOverlap(Box)
  (params (OverlappedComponent :type Primitive%20Component%20Object%20Reference) (OtherActor :type Actor%20Object%20Reference) (OtherComp :type Primitive%20Component%20Object%20Reference) (OtherBodyIndex :type Integer) (bFromSweep :type Boolean) (SweepResult :type Hit%20Result%20Structure%20%28by%20ref%29))
  (bind (_asbp_boat_char _bsuccess) (Utilities|Casting|CastToBP_BoatChar OtherActor))
  (bind _meshcomp (Variables|/Script/MetaverseXRTest.MXR_BoatChar|GetMeshComp _asbp_boat_char))
  (bind _returnvalue (Transformation|GetWorldRotation _meshcomp))
  (if (and _bsuccess (<= (Math|Vector|VectorLength (Transformation|GetVelocity OtherActor)) 1.5e+03))
    (if (and (>= (.yaw _returnvalue) -25.0) (<= (.yaw _returnvalue) 25.0))
      (bind _returnvalue_2 (Utilities|Time|SetTimerbyEvent (delegate Custom|TimeElapsed) 5.0))
      (Variables|Default|SetTimer%20Ref _returnvalue_2)
      (Variables|Default|SetPlayerReference 0)
      (Development|PrintString "Waiting..")
      (bind _returnvalue_3 (Niagara|SpawnSystematLocation "/Game/Particles/Stage/NS_WinParticles.NS_WinParticles" (Transformation|GetActorLocation) "0, 0, 0" "1.000000,1.000000,1.000000" false))
      (Variables|Default|SetParticleRef _returnvalue_3))))

(event OnComponentEndOverlap(Box)
  (params (OverlappedComponent :type Primitive%20Component%20Object%20Reference) (OtherActor :type Actor%20Object%20Reference) (OtherComp :type Primitive%20Component%20Object%20Reference) (OtherBodyIndex :type Integer))
  (if (Utilities|IsValid (.AsBP%20Boat%20Char (Utilities|Casting|CastToBP_BoatChar OtherActor)))
    (Utilities|Time|ClearandInvalidateTimerbyHandle (Variables|Default|GetTimer%20Ref))
    (Components|DestroyComponent (Variables|Default|GetParticleRef))))

(event Custom|TimeElapsed
  (Default|ShowWidget (.AsBP%20Game%20HUD (Utilities|Casting|CastToBP_GameHUD (HUD|GetHUD (Game|GetPlayerController 0)))) "/Game/Blueprints/UMG/UMG_WinScreen.UMG_WinScreen_C"))

(fn ConstructionScript)